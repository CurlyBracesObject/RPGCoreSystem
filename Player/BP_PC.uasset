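; BP_PC is the player controller that handles the switch from the start pawn into the Frozen Cove level.
; BeginPlay caches the BP_StartPawn.
; LevelChange stream-loads Frozen Cove with blocking, tells BP_HUD to show the main UI, then spawns and possesses BP_Gideon at a PlayerStart and destroys the start pawn.
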(event `self.ReceiveBeginPlay`
  (bind _asbp_start_pawn (cast `/Game/ThirdPersonGame/Player/BP_StartPawn` (`GameplayStatics.GetPlayerPawn` 0)))
  (set `self.StartPawn` _asbp_start_pawn))

(event `LevelChange`
  (`GameplayStatics.LoadStreamLevelBySoftObjectPtr` "/Game/InfinityBladeIceLands/Maps/FrozenCove.FrozenCove" true true)
  (`|ExecutionSequence`
    (:`then_0`
      (bind _asbp_hud (cast `/Game/ThirdPersonGame/Player/BP_HUD` (`self.GetHUD`)))
      (`/Game/ThirdPersonGame/Player/BP_HUD.ShowMainUI` _asbp_hud))
    (:`then_1`
      (bind _returnvalue (`GameplayStatics.GetActorOfClass` "/Script/Engine.PlayerStart"))
      (bind _returnvalue_2 (`|SpawnActorFromClass` "/Game/ThirdPersonGame/Player/BP_Gideon.BP_Gideon_C" (`self.GetTransform` _returnvalue) "Undefined" "OverrideRootScale" null null))
      (`self.Possess` _returnvalue_2)
      (`self.K2_DestroyActor` (`self.StartPawn`)))))

(fn `UserConstructionScript`)