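; BP_Gideon is the playable character, with walk, run, standstill-only jump and clamped HP damage.
; Left click plays a spell montage, or casts the Q-toggled skill by replacing its targeting decal with a damage actor at the aim point.
; Each Tick, a camera trace updates that point, highlights the aimed BP_AI via custom depth and recolors the crosshair.
; Skill cooldown comes from GameState data and drives a HUD gradient.
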(event `InputAxis|MoveRight`
  (params (AxisValue :type "Float (single-precision)"))
  ;[1 1 1] PlayerMovement
  (`self.AddMovementInput` (`KismetMathLibrary.GetRightVector` (`KismetMathLibrary.MakeRotator` 0.0 0.0 (.yaw (`self.GetControlRotation`)))) AxisValue))

(event `InputAxis|MoveForward`
  (params (AxisValue :type "Float (single-precision)"))
  ;[1 1 1] PlayerMovement
  (`self.AddMovementInput` (`KismetMathLibrary.GetForwardVector` (`KismetMathLibrary.MakeRotator` 0.0 0.0 (.yaw (`self.GetControlRotation`)))) AxisValue))

(event `InputAxis|TurnRight`
  (params (AxisValue :type "Float (single-precision)"))
  ;[1 1 1] PlayerMovement
  (`self.AddControllerYawInput` AxisValue))

(event `InputAxis|LookUp`
  (params (AxisValue :type "Float (single-precision)"))
  ;[1 1 1] PlayerMovement
  (if true
    (`self.AddControllerPitchInput` (* AxisValue -1.0))))

(event `InputAction|Jump`
  (params (Key :type "Key Structure"))
  ;[1 1 1] PlayerMovement
  (:`Pressed`
    (if (== (`MovementComponent.Velocity` (`self.CharacterMovement`)) (0.0 0.0 0.0))
      (`self.Jump`))))

(event `InputAction|Run`
  (params (Key :type "Key Structure"))
  (bind _charactermovement (`self.CharacterMovement`))
  ;[1 1 1] PlayerMovement
  (:`Pressed`
    (set `CharacterMovementComponent.MaxWalkSpeed` 600.0 _charactermovement))
  (:`Released`
    (set `CharacterMovementComponent.MaxWalkSpeed` 375.0 _charactermovement)))

(event `InputAction|LeftMouseKey_SpellAttack`
  (params (Key :type "Key Structure"))
  ;[1 1 1] PlayerAttack
  (:`Pressed`
    (if (not (`self.IsAttack`))
      (set `self.IsAttack` true)
      (switch `int` (`self.SkillIndex`)
        (:`0`
          (bind _returnvalue (`self.PlayAnimMontage` "/Game/ThirdPersonGame/Player/Animations/GideonAnim/AnimMontage_GideonSpellAttack.AnimMontage_GideonSpellAttack"))
          (`KismetSystemLibrary.Delay` _returnvalue)
          (`self.ReturnValue`))
        (:`1`
          (if (not (`self.IsCDTime`))
            (set `self.IsCDTime` true)
            (`self.CallSkillUICDGradient`)
            (`|SpawnActorFromClass` "/Game/ThirdPersonGame/Actor/BP_DamageActor.BP_DamageActor_C" (`KismetMathLibrary.MakeTransform` (`self.HitLocation`)) "Undefined" "OverrideRootScale" null null)
            (`self.K2_DestroyActor` (`self.DecalActor`))
            (`KismetSystemLibrary.Delay` (/ (`.CDTime_7_F62EBDC74DDEE3F3D25C6B8718AFAD9B` (break `/Game/ThirdPersonGame/Data/Struct_SkillInfo` (`self.SkillInfo` 0))) 2.0))
            (`|ExecutionSequence`
              (:`then_0`
                (set `self.IsCDTime` false))
              (:`then_1`
                (`self.ReturnValue`))
              (:`then_2`
                (set `self.CurrentCD` (`.CDTime_7_F62EBDC74DDEE3F3D25C6B8718AFAD9B` (break `/Game/ThirdPersonGame/Data/Struct_SkillInfo` (`self.SkillInfo` 0))))))))))))

(event `ReturnValue`
  ;[1 1 1] PlayerAttack
  (set `self.SkillIndex` 0)
  (set `self.IsAttack` false))

(event `InputAction|QKey_SkillAAttack`
  (params (Key :type "Key Structure"))
  (:`Pressed`
    (if (`self.IsAttack`)
      _
      (elif (`AnimInstance.IsAnyMontagePlaying` (`SkeletalMeshComponent.GetAnimInstance` (`self.Mesh`)))
        _
        (elif (>= (`self.CurrentCD`) (`.CDTime_7_F62EBDC74DDEE3F3D25C6B8718AFAD9B` (break `/Game/ThirdPersonGame/Data/Struct_SkillInfo` (`self.SkillInfo` 0))))
          ;[1 1 1] PlayerAttack
          (if (`self.IsCDTime`)
            _
            (elif (== (`self.SkillIndex`) 0)
              (set `self.SkillIndex` 1)
              (bind _returnvalue (`|SpawnActorFromClass` "/Game/ThirdPersonGame/Actor/BP_Decal.BP_Decal_C" (`KismetMathLibrary.MakeTransform` (`self.HitLocation`)) "Undefined" "OverrideRootScale" null null))
              (set `self.DecalActor` _returnvalue)
              (else
                (set `self.SkillIndex` 0)
                (`self.K2_DestroyActor` (`self.DecalActor`))))))))))

(event `self.ReceiveAnyDamage`
  (params (Damage :type "Float (single-precision)") (DamageType :type "DamageType Object Reference") (InstigatedBy :type "Controller Object Reference") (DamageCauser :type "Actor Object Reference"))
  ;[1 1 1] EventAnyDamage
  (set `self.CurrentHP` (`KismetMathLibrary.FClamp` (- (`self.CurrentHP`) Damage) 0.0 (`self.MaxHP`))))

(event `self.ReceiveTick`
  (params (DeltaSeconds :type "Float (single-precision)"))
  (bind _aiactor (`self.AIActor`))
  ;[1 1 1] CreateCrossshair
  (bind (_isreachcertainplace _hitlocation _hitactor) (`self.LineTraceTick`))
  (if _isreachcertainplace
    (set `self.HitLocation` _hitlocation)
    (bind _asbp_ai (cast `/Game/ThirdPersonGame/Enemy/BP_AI` _hitactor)
      (:`then`
        (`/Engine/EditorBlueprintResources/StandardMacros.IsValid` _aiactor
          (:`Is Valid`
            (if (not (== _aiactor _asbp_ai))
              (`self.SetAIRenderDepth` false)
              (set `self.AIActor` null)
              (set `self.AIActor` _asbp_ai :!label _label)
              (`self.SetAIRenderDepth` true)
              (`|ExecutionSequence`
                (:`then_0`
                  (`/Engine/EditorBlueprintResources/StandardMacros.DoOnce` false :!label _label_2
                    (:`Completed`
                      (`/Game/ThirdPersonGame/UI/UI_MainUI.CrosshairColorChange` (`self.GetMainUIFunc`) "Forward"))))
                (:`then_1`
                  (goto _label_4 :!via `Reset`)))))
          (:`Is Not Valid`
            (goto _label))))
      (:`CastFailed`
        (`self.SetAIRenderDepth` false :!label _label_3)
        (set `self.AIActor` null)
        (`|ExecutionSequence`
          (:`then_0`
            (`/Engine/EditorBlueprintResources/StandardMacros.DoOnce` false :!label _label_4
              (:`Completed`
                (`/Game/ThirdPersonGame/UI/UI_MainUI.CrosshairColorChange` (`self.GetMainUIFunc`) "Reverse"))))
          (:`then_1`
            (goto _label_2 :!via `Reset`)))))
    (else
      (set `self.HitLocation` (0.0 0.0 0.0))
      (goto _label_3))))

(event `self.ReceiveBeginPlay`)

(fn `CallSkillUICDGradient`
  (`/Game/ThirdPersonGame/UI/UI_SkillUI.SkillUIGradientCDTime` (`|GetArrayItem` (`/Game/ThirdPersonGame/UI/UI_MainUI.SkillUIButton` (`/Game/ThirdPersonGame/Player/BP_HUD.MainUI` (cast `/Game/ThirdPersonGame/Player/BP_HUD` (`PlayerController.GetHUD` (`GameplayStatics.GetPlayerController` 0)) :!pure true))) (- (`self.SkillUIIndex`) 0))))

(fn `GetMainUIFunc`
  (returns (MainUI :type "/Game/ThirdPersonGame/UI/UI_MainUI Object Reference"))
  (bind _asbp_hud (cast `/Game/ThirdPersonGame/Player/BP_HUD` (`PlayerController.GetHUD` (`GameplayStatics.GetPlayerController` 0))))
  (return (`/Game/ThirdPersonGame/Player/BP_HUD.MainUI` _asbp_hud)))

(fn `LineTraceTick`
  (returns (IsReachCertainPlace :type Boolean) (HitLocation :type "Vector Structure") (HitActor :type "Actor Object Reference"))
  (bind _returnvalue (`GameplayStatics.GetPlayerCameraManager` 0))
  (bind _returnvalue_2 (`self.K2_GetActorLocation` _returnvalue))
  (bind (_outhit _returnvalue_3) (`KismetSystemLibrary.LineTraceSingleForObjects` :`Start` _returnvalue_2 :`End` (+ _returnvalue_2 (* (`self.GetActorForwardVector` _returnvalue) 5000)) :`ObjectTypes` (`|MakeArray` "ObjectTypeQuery1" "ObjectTypeQuery2" "ObjectTypeQuery7" :!type "EObjectTypeQuery Enum") :`DrawDebugType` "ForOneFrame"))
  (bind (_bblockinghit _binitialoverlap _time _distance _location _impactpoint _normal _impactnormal _physmat _hitactor) (`GameplayStatics.BreakHitResult` _outhit))
  (return _returnvalue_3 _location _hitactor))

(fn `SetAIRenderDepth`
  (params (IsRender :type Boolean))
  (bind _aiactor (`self.AIActor`))
  (`/Engine/EditorBlueprintResources/StandardMacros.IsValid` _aiactor
    (:`Is Valid`
      (`|ExecutionSequence`
        (:`then_0`
          (for _array_element (`self.K2_GetComponentsByClass` _aiactor "/Script/Engine.StaticMeshComponent")
            (`PrimitiveComponent.SetRenderCustomDepth` _array_element IsRender)))
        (:`then_1`
          (for _array_element_2 (`self.K2_GetComponentsByClass` _aiactor "/Script/Engine.SkeletalMeshComponent")
            (`PrimitiveComponent.SetRenderCustomDepth` _array_element_2 IsRender)))))))

(fn `SkillInfo`
  (params (SkillIndexGetSkillStructInfo :type Integer))
  (returns (StructSkillInfo :type "/Game/ThirdPersonGame/Data/Struct_SkillInfo Structure"))
  (return (`|GetArrayItem` (`.Skill_23_6E9F924C43565770830020B0EE2931D9` (break `/Game/ThirdPersonGame/Data/Struct_PlayerInfo` (`|GetArrayItem` (`/Game/ThirdPersonGame/Player/BP_GameStateBase.PlayerInfo` (cast `/Game/ThirdPersonGame/Player/BP_GameStateBase` (`GameplayStatics.GetGameState`) :!pure true))))))))

(fn `UserConstructionScript`)