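; Player character Blueprint for the Assassin Lady, handling movement, camera look, run, jump and an attack.
; Input axes drive movement and view, Run switches walk speed, and Jump only fires from a standstill.
; SpellAttack plays an attack montage, with a flag and montage-length delay blocking re-triggering.
; The construction script links modular hair, gauntlet, head, body, mask and shoe meshes to the main mesh via master pose.
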(event `InputAxis|MoveForward`
  (params (AxisValue :type "Float (single-precision)"))
  ;[1 1 1] PlayerMovement
  (`self.AddMovementInput` (`self.GetActorForwardVector`) AxisValue))

(event `InputAxis|MoveRight`
  (params (AxisValue :type "Float (single-precision)"))
  ;[1 1 1] PlayerMovement
  (`self.AddMovementInput` (`self.GetActorRightVector`) AxisValue))

(event `InputAxis|TurnRight`
  (params (AxisValue :type "Float (single-precision)"))
  ;[1 1 1] PlayerMovement
  (`self.AddControllerYawInput` AxisValue))

(event `InputAxis|LookUp`
  (params (AxisValue :type "Float (single-precision)"))
  ;[1 1 1] PlayerMovement
  (`self.AddControllerPitchInput` (* AxisValue -1.0)))

(event `InputAction|Jump`
  (params (Key :type "Key Structure"))
  ;[1 1 1] PlayerMovement
  (:`Pressed`
    (if (== (`MovementComponent.Velocity` (`self.CharacterMovement`)) (0.0 0.0 0.0))
      (`self.Jump`))))

(event `InputAction|Run`
  (params (Key :type "Key Structure"))
  (bind _charactermovement (`self.CharacterMovement`))
  ;[1 1 1] PlayerMovement
  (:`Pressed`
    (set `CharacterMovementComponent.MaxWalkSpeed` 600.0 _charactermovement))
  (:`Released`
    (set `CharacterMovementComponent.MaxWalkSpeed` 375.0 _charactermovement)))

(event `InputAction|SpellAttack`
  (params (Key :type "Key Structure"))
  ;[1 1 1] PlayerAttack
)

(event `InputAction|SpellAttack`
  (params (Key :type "Key Structure"))
  ;[1 1 1] PlayerAttack
  (:`Pressed`
    (if (not (`self.IsAttack`))
      (set `self.IsAttack` true)
      (bind _returnvalue (`self.PlayAnimMontage` "/Game/ThirdPersonGame/Player/Animations/AssassinLadyAnim/AnimMontage_AssassinAttack1.AnimMontage_AssassinAttack1"))
      (`KismetSystemLibrary.Delay` _returnvalue)
      (set `self.IsAttack` false))))

(fn `UserConstructionScript`
  (`SkinnedMeshComponent.SetLeaderPoseComponent` (`self.SK_Hair4HoodB`) (`self.Mesh`) false)
  (`SkinnedMeshComponent.SetLeaderPoseComponent` (`self.SK_GauntletA_L`) (`self.Mesh`) false)
  (`SkinnedMeshComponent.SetLeaderPoseComponent` (`self.SK_GauntletA_R`) (`self.Mesh`) false)
  (`SkinnedMeshComponent.SetLeaderPoseComponent` (`self.SK_HeadA`) (`self.Mesh`) false)
  (`SkinnedMeshComponent.SetLeaderPoseComponent` (`self.SK_TopBodyC`) (`self.Mesh`) false)
  (`SkinnedMeshComponent.SetLeaderPoseComponent` (`self.SK_Mask`) (`self.Mesh`) false)
  (`SkinnedMeshComponent.SetLeaderPoseComponent` (`self.SK_Shoes`) (`self.Mesh`) false))