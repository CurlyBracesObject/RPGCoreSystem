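; BP_Decal is an actor that follows the aim point of the player's BP_Gideon character, apparently as a skill targeting marker.
; Each tick it casts the player character to BP_Gideon and moves itself to that character's HitLocation without sweep.
; An unconnected branch would spawn BP_DamageActor at the decal and destroy it when SkillIndex is zero, but it never runs.
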(event `self.ReceiveTick`
  (params (DeltaSeconds :type "Float (single-precision)"))
  (`self.K2_SetActorLocation` (`/Game/ThirdPersonGame/Player/BP_Gideon.HitLocation` (cast `/Game/ThirdPersonGame/Player/BP_Gideon` (`GameplayStatics.GetPlayerCharacter` 0) :!pure true))))

(fn `UserConstructionScript`)