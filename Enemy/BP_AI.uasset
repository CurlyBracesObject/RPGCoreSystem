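; Enemy AI character that takes and deals damage, shows a floating health bar and registers itself on the player's minimap.
; AnyDamage lowers clamped HP, and a custom event deals fixed damage to the player character.
; While the HP widget is visible, Tick turns it toward the camera and checks for death.
; Death sets the blackboard flag, plays an animation, disables capsule collision, removes the minimap marker and hides the widget, ending the checks.
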(event `self.ReceiveAnyDamage`
  (params (Damage :type "Float (single-precision)") (DamageType :type "DamageType Object Reference") (InstigatedBy :type "Controller Object Reference") (DamageCauser :type "Actor Object Reference"))
  (set `self.AICurrentHP` (`KismetMathLibrary.FClamp` (- (`self.AICurrentHP`) Damage) 0.0 (`self.AIMaxHP`))))

(event `self.ReceiveBeginPlay`
  (`|ExecutionSequence`
    (:`then_0`
      ;[1 1 1] CreateAIUIHP
      (bind _asui_aihpui (cast `/Game/ThirdPersonGame/UI/UI_AIHPUI` (`WidgetComponent.GetUserWidgetObject` (`self.AIHPWidget`))))
      (set `/Game/ThirdPersonGame/UI/UI_AIHPUI.AIActor` self _asui_aihpui))
    (:`then_1`
      (`KismetSystemLibrary.Delay` 0.2)
      (bind _asbp_hud (cast `/Game/ThirdPersonGame/Player/BP_HUD` (`PlayerController.GetHUD` (`GameplayStatics.GetPlayerController` 0))))
      (`/Game/ThirdPersonGame/UI/UI_MiniMap.AddAILocationUI` (`/Game/ThirdPersonGame/UI/UI_MainUI.UI_MiniMap` (`/Game/ThirdPersonGame/Player/BP_HUD.MainUI` _asbp_hud)) self))))

(event `self.ReceiveTick`
  (params (DeltaSeconds :type "Float (single-precision)"))
  (bind _aihpwidget (`self.AIHPWidget`))
  (if (`SceneComponent.IsVisible` _aihpwidget)
    (`SceneComponent.K2_SetWorldRotation` _aihpwidget (`KismetMathLibrary.FindLookAtRotation` (`SceneComponent.K2_GetComponentLocation` (`self.AIHPWidget`)) (`self.K2_GetActorLocation` (`GameplayStatics.GetPlayerCameraManager` 0))) false false)
    (`self.LogicafterAIDeath`)))

(event `ApplayDamagetoPlayerCharacter`
  (bind _returnvalue (`GameplayStatics.ApplyDamage` (`GameplayStatics.GetPlayerCharacter` 0) 5.0 null self)))

(fn `LogicafterAIDeath`
  (if (== (`self.AICurrentHP`) 0.0)
    (`BlackboardComponent.SetValueAsBool` (`AIBlueprintHelperLibrary.GetBlackboard` null) (`self.IsDeath`) true)
    (`SkeletalMeshComponent.PlayAnimation` (`self.Mesh`) (`self.DeathAnimSequence`) false)
    (`SceneComponent.SetVisibility` (`self.AIHPWidget`) false false)
    (`PrimitiveComponent.SetCollisionEnabled` (`self.CapsuleComponent`) "NoCollision")
    (bind _asbp_hud (cast `/Game/ThirdPersonGame/Player/BP_HUD` (`PlayerController.GetHUD` (`GameplayStatics.GetPlayerController` 0))))
    (`/Game/ThirdPersonGame/UI/UI_MiniMap.RemoveAILocationUI` (`/Game/ThirdPersonGame/UI/UI_MainUI.UI_MiniMap` (`/Game/ThirdPersonGame/Player/BP_HUD.MainUI` _asbp_hud)) self)))

(fn `UserConstructionScript`)